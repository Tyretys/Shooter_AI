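; AI controller for SWAT characters that runs the BT_SWAT_Main behavior tree and feeds it perception results through the blackboard.
; The main perception component routes stimuli by sense class through HandleSenses.
; Sight sets enemy visibility and the target actor, swapping it for the last stimulus location when lost, while hearing flags investigation and records the noise location.
; A second, peripheral perception component writes visibility and target actor directly, without clearing the target on loss.
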(event OnTargetPerceptionUpdated(AIPerception)
  (params (Actor :type Actor%20Object%20Reference) (Stimulus :type AI%20Stimulus%20Structure))
  (bind _output_get (Variables|Default|SetStimulus Stimulus))
  (bind _returnvalue (Class|AIPerceptionSystem|GetSenseClassforStimulus _output_get))
  (CallFunction|HandleSenses (Utilities|GetClassDisplayName _returnvalue) Actor))

(event OnTargetPerceptionUpdated(AIPerception_peripheral)
  (params (Actor :type Actor%20Object%20Reference) (Stimulus :type AI%20Stimulus%20Structure))
  (AI|Components|Blackboard|SetValueasBool (AI|GetBlackboard 0) (Utilities|Name|MakeLiteralName "isEnemyVisisble?") (.bSuccessfullySensed (Utilities|Struct|BreakAIStimulus Stimulus)))
  (AI|Components|Blackboard|SetValueasObject (AI|GetBlackboard 0) (Utilities|Name|MakeLiteralName "TargetActor") Actor))

(event EventBeginPlay
  (AI|RunBehaviorTree "/Game/MyBlueprints/AI/Blueprints/BT/BT_SWAT_Main.BT_SWAT_Main"))

(fn ConstructionScript)

(fn HandleSenses
  (params (Selection :type String) (Sensed%20Actor :type Actor%20Object%20Reference))
  (bind _stimulus (Variables|Default|GetStimulus))
  (bind _stimulus_2 (Variables|Default|GetStimulus))
  (switch string Selection
    (:AISense_Sight
      (AI|Components|Blackboard|SetValueasBool (AI|GetBlackboard 0) (Utilities|Name|MakeLiteralName "isEnemyVisisble?") (.bsuccessfullysensed _stimulus_2))
      (if (.bsuccessfullysensed _stimulus_2)
        (AI|Components|Blackboard|SetValueasObject (AI|GetBlackboard 0) (Utilities|Name|MakeLiteralName "TargetActor") Sensed%20Actor)
        (else
          (AI|Components|Blackboard|ClearValue (AI|GetBlackboard 0) (Utilities|Name|MakeLiteralName "TargetActor"))
          (AI|Components|Blackboard|SetValueasVector (AI|GetBlackboard 0) (Utilities|Name|MakeLiteralName "TargetLocation") (.stimuluslocation (Variables|Default|GetStimulus))))))
    (:AISense_Hearing
      (AI|Components|Blackboard|SetValueasBool (AI|GetBlackboard 0) (Utilities|Name|MakeLiteralName "isInvestigating?") (.bsuccessfullysensed _stimulus))
      (if (.bsuccessfullysensed _stimulus)
        (AI|Components|Blackboard|SetValueasVector (AI|GetBlackboard 0) (Utilities|Name|MakeLiteralName "TargetLocation") (.stimuluslocation (Variables|Default|GetStimulus)))))))