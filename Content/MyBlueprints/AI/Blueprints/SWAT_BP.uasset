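; SWAT AI character that shoots and lobs grenades at the player, with crouch events and a hit-reaction montage on damage.
; It attaches its primary weapon to a hand socket and writes its location to the Blackboard on a looping timer.
; Bullets spawn at the muzzle socket facing the player.
; Grenades target a random reachable point near the player, solving the high-arc launch angle from projectile-motion math and printing a message when out of range.
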(event Custom|Event%20Fire_bullet
  (bind _self self)
  (bind _returnvalue (Actor|GetComponentbyClass _self "/Script/Engine.SkeletalMeshComponent"))
  (bind _returnvalue_2 (Transformation|GetSocketTransform _returnvalue "muzzle_socket" "RTS_World"))
  (Game|SpawnActorfromClass "/Game/MyBlueprints/AI/Blueprints/Bullet_BP.Bullet_BP_C" (Math|Transform|MakeTransform (.location _returnvalue_2) (Math|Rotator|FindLookatRotation (.location _returnvalue_2) (Transformation|GetActorLocation (Game|GetPlayerCharacter 0))) (.scale _returnvalue_2)) "AdjustIfPossibleButAlwaysSpawn" 0 self))

(event Custom|SetSelfPosition
  (AI|Components|Blackboard|SetValueasVector (AI|GetBlackboard 0) (Utilities|Name|MakeLiteralName "SelfPosition") (Transformation|GetActorLocation)))

(event Custom|ThrowGrenade
  (Variables|GrenadeThrow|SetSelfLocation (Transformation|GetActorLocation))
  (Variables|Default|SetGrenadeStart (Transformation|GetSocketLocation (Actor|GetComponentbyClass self "/Script/Engine.SkeletalMeshComponent") "GrenadeSocket"))
  (Variables|GrenadeThrow|SetTargetVector (.RandomLocation (AI|Navigation|GetRandomReachablePointinRadius (Transformation|GetActorLocation (Game|GetPlayerCharacter 0)) 2.5e+02 0 0)))
  (CallFunction|CalculateAngleandSpawnGreande))

(event EventBeginPlay
  ;[1 1 1] Initialy attach weapon to hand socket
  (bind _output_get (Variables|Default|SetCurrentWeapon (Variables|/Script/Engine.ChildActorComponent|GetChildActor (Variables|Default|GetPrimaryWeapon))))
  (Transformation|AttachComponentToComponent _output_get (Variables|Character|GetMesh) "WeaponSocket" "SnapToTarget" "SnapToTarget" "SnapToTarget" true)
  (Utilities|Time|SetTimerbyEvent (delegate Custom|SetSelfPosition) 0.5 true))

(event Game|Damage|EventAnyDamage
  (params (Damage :type Float%20%28single-precision%29) (DamageType :type Damage%20Type%20Object%20Reference) (InstigatedBy :type Controller%20Object%20Reference) (DamageCauser :type Actor%20Object%20Reference))
  (Animation|Montage|PlayMontage (Variables|Character|GetMesh) "/Game/SWAT/Animations/Montages/hit_reaction_Montage.hit_reaction_Montage"))

(event EventAICrouch
  (Character|Crouch))

(event EventAIUnCrouch
  (Character|UnCrouch))

(fn ConstructionScript)

(fn CalculateAngleandSpawnGreande
  (bind _selflocation (Variables|GrenadeThrow|GetSelfLocation))
  (bind _targetvector (Variables|GrenadeThrow|GetTargetVector))
  (bind _selflocation_2 (Variables|GrenadeThrow|GetSelfLocation))
  (bind _targetvector_2 (Variables|GrenadeThrow|GetTargetVector))
  (bind _returnvalue (Math|Rotator|FindLookatRotation _selflocation_2 _targetvector))
  (bind _returnvalue_2 (- (.x _targetvector_2) (.x _selflocation)))
  (bind _returnvalue_3 (- (.y _targetvector_2) (.y _selflocation)))
  (bind _returnvalue_4 (Math|Vector2D|Vector2DLength (Math|Vector2D|MakeVector2D _returnvalue_2 _returnvalue_3)))
  (bind _output_get (Variables|GrenadeThrow|SetVelocity^2 (Math|Float|Square (Variables|GrenadeThrow|GetVelocity))))
  (Variables|GrenadeThrow|SetVelocity^4 (Math|Float|Square _output_get))
  (if (>= (- (Variables|GrenadeThrow|GetVelocity^4) (* (+ (* (Math|Float|Square _returnvalue_4) (Variables|GrenadeThrow|GetGravity)) (* (* (- (.z _targetvector_2) (.z _selflocation)) (Variables|GrenadeThrow|GetVelocity^2)) 2.0)) (Variables|GrenadeThrow|GetGravity))) 0.0)
    (Game|SpawnActorfromClass "/Game/MyBlueprints/AI/Blueprints/Grenade_BP.Grenade_BP_C" (Math|Transform|MakeTransform (Variables|Default|GetGrenadeStart) (Math|Rotator|MakeRotator (.roll _returnvalue) (Class|KismetMathLibrary|DegAtan (/ (+ (Math|Float|Sqrt (- (Variables|GrenadeThrow|GetVelocity^4) (* (+ (* (Math|Float|Square _returnvalue_4) (Variables|GrenadeThrow|GetGravity)) (* (* (- (.z _targetvector_2) (.z _selflocation)) (Variables|GrenadeThrow|GetVelocity^2)) 2.0)) (Variables|GrenadeThrow|GetGravity)))) (Variables|GrenadeThrow|GetVelocity^2)) (* _returnvalue_4 (Variables|GrenadeThrow|GetGravity)))) (.yaw _returnvalue)) "2.000000,2.000000,2.000000") "AlwaysSpawn" 0 self)
    (else
      (Development|PrintString (Utilities|String|Append "Unreacheble Angle:" (Utilities|String|ToString(Float) (Variables|GrenadeThrow|GetVelocity^4))) true true "(R=1.000000,G=0.009454,B=0.000000,A=1.000000)"))))